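; Enemy Blueprint that wanders at random and dies to a single hit.
; From BeginPlay, a self-calling roam event sends it via AI MoveTo to a random reachable nearby point, picking a new one after a short delay from the immediate exec pin, without waiting for arrival.
; Any damage sets Health to zero regardless of amount, destroying the actor and printing a placeholder string; the damage subtraction is left unconnected.
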(event `self.ReceiveBeginPlay`
  (`self.Roam aound`))

(event `Roam aound`
  (`|AIMoveTo` self (`NavigationSystemV1.K2_GetRandomReachablePointInRadius` (`self.K2_GetActorLocation`) 2000.0 null null) null 120.0
    (:`then`
      (`KismetSystemLibrary.Delay` 1.2)
      (`self.Roam aound`))))

(event `self.ReceiveAnyDamage`
  (params (Damage :type "Float (single-precision)") (DamageType :type "DamageType Object Reference") (InstigatedBy :type "Controller Object Reference") (DamageCauser :type "Actor Object Reference"))
  (bind _output_get (set `self.Health` 0.0))
  (if (<= (`self.Health`) 0.0)
    (`self.K2_DestroyActor`)
    (`KismetSystemLibrary.PrintString` "fwrgfwsrggsrg")))

(fn `UserConstructionScript`)